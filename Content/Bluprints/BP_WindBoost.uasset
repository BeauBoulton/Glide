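; BP_WindBoost is a wind boost actor that repeatedly pushes overlapping actors implementing BPI_Pushable.
; On overlap begin it sends OnEnterBoostMessage, repeating every BoostLoopTime until any overlap ends and sets BreakLoop.
; TraceForPlayer sphere-traces from above the Cylinder to BoostRange along its up vector, returning a pushable hit with debug prints.
; The event graph never calls this trace.
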(event `self.ReceiveActorBeginOverlap`
  (params (OtherActor :type "Actor Object Reference"))
  (set `self.BreakLoop` false)
  (if (`KismetSystemLibrary.DoesImplementInterface` OtherActor "/Game/Bluprints/Interfaces/BPI_Pushable.BPI_Pushable_C") :!label _label
    (message `/Game/Bluprints/Interfaces/BPI_Pushable.OnEnterBoost` OtherActor self)
    (`KismetSystemLibrary.Delay` (`self.BoostLoopTime`))
    (if (not (`self.BreakLoop`))
      (goto _label))))

(event `self.ReceiveActorEndOverlap`
  (params (OtherActor :type "Actor Object Reference"))
  (set `self.BreakLoop` true))

(fn `GetMaxHeightPoint`
  (params (Target :type "SceneComponent Object Reference"))
  (returns (ReturnValue :type "Vector Structure"))
  (return (+ (`SceneComponent.K2_GetComponentLocation` Target) (* (`SceneComponent.GetUpVector` Target) (`self.BoostRange`)))))

(fn `UserConstructionScript`)