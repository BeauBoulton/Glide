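; BP_CheckpointManager tracks how far the player has progressed through a level's checkpoints.
; On BeginPlay it counts all Bp_Checkpoint actors and caches a reference to the BP_LevelEnd actor.
; Each CheckpointGet call decrements the remaining count and, unless the level is complete, recalculates LevelProgress as a percentage.
; The divisor is total checkpoints plus one, so collecting every checkpoint alone stays short of 100%.
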(event `self.ReceiveBeginPlay`
  ;[0 0 0 0.5] Get all checkpoints in level and set checkpoint count
  (`|ExecutionSequence`
    (:`then_0`
      (bind _outactors (`GameplayStatics.GetAllActorsOfClass` "/Game/Bluprints/Checkpoint/Bp_Checkpoint.Bp_Checkpoint_C"))
      (bind _output_get (set `self.TotalCheckpointCount` (`KismetArrayLibrary.Array_Length` _outactors)))
      (set `self.CurrentCheckpointCount` _output_get))
    (:`then_1`
      ;[0 0 0 0.5] Get reference to level end
      (bind _returnvalue (`GameplayStatics.GetActorOfClass` "/Game/Bluprints/Checkpoint/BP_LevelEnd.BP_LevelEnd_C"))
      (set `self.LevelEnd` _returnvalue))))

(event `CheckpointGet`
  (bind _returnvalue (`KismetMathLibrary.Conv_IntToDouble` (+ (`self.TotalCheckpointCount`) 1)))
  ;[0 0 0 0.5] Decrement checkpoint count when player gets a new checkpoint
  (`/Engine/EditorBlueprintResources/StandardMacros.DecrementInt` (`self.CurrentCheckpointCount`)
    (:`  `
      (if (not (`/Game/Bluprints/Checkpoint/BP_LevelEnd.LevelComplete` (`self.LevelEnd`)))
        (set `self.Level Progress` (* (/ (- _returnvalue (`KismetMathLibrary.Conv_IntToDouble` (+ (`self.CurrentCheckpointCount`) 1))) _returnvalue) 100.0))))))

(fn `UserConstructionScript`)